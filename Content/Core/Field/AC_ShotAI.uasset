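; Actor component on BP_GameState that acts as the shooting AI in a Battleship-style grid game.
; AIFire requests a cell, fires through BPMainField and recursively retries when the cell or shot is invalid.
; Easy picks random cells; Normal also does until a hit, then probes shuffled directions from it.
; The field's OnShot event updates that targeting, dropping perpendicular directions on further hits and clearing it once the ship sinks.
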(event `self.ReceiveBeginPlay`
  (bind _asbp_game_state (cast `/Game/Core/BP_GameState` (`self.GetOwner`)))
  (bind _bp_mainfield (`/Game/Core/BP_GameState.BP_MainField` _asbp_game_state)
    (:`then`
      (add `/Game/Core/Field/BP_ParentField.OnShot` _bp_mainfield (delegate `CustomEvent`)))
    (:`else`
      (`KismetSystemLibrary.PrintString` "Error: MainField empty (AC_ShptAI)" true true (struct :`R` 1.0 :`A` 1.0) 10.0))))

(event `CustomEvent`
  (params (Field :type "/Game/Core/Field/BP_ParentField Object Reference") (`Hit?` :type Boolean) (ShipDestroyed :type Boolean))
  (bind _array (`|MakeArray` "Left" "Right" :!type "ETouchSwipeDirection Enum"))
  (bind _array_2 (`|MakeArray` "Up" "Down" :!type "ETouchSwipeDirection Enum"))
  (cast `/Game/Core/Field/BP_MainField` Field)
  (bind _asbp_battle_game_mode (cast `/Game/Core/BP_BattleGameMode` (`GameplayStatics.GetGameMode`)))
  (switch `/Game/Core/Enums/E_Difficulty` (`/Game/Core/BP_BattleGameMode.GameDifficulty` _asbp_battle_game_mode)
    (:`NewEnumerator0`
      (if `Hit?`
        _))
    (:`NewEnumerator2`
      (`self.HittedShip`
        (:`then`
          (if ShipDestroyed
            (set `self.HittedShip` null)
            (elif `Hit?`
              (for _array_element (select `ETouchSwipeDirection` (`|GetArrayItem` (`self.DirectionToFire`)) :`Left` _array_2 :`Right` _array_2 :`Up` _array :`Down` _array)
                (`KismetArrayLibrary.Array_RemoveItem` (`self.DirectionToFire`) _array_element))
              (else
                (`KismetArrayLibrary.Array_Remove` (`self.DirectionToFire`))
                (set `self.TempPos` (`self.HittedPos`))))))
        (:`else`
          (if `Hit?`
            (set `self.HittedPos` (`self.NextCellPos`))
            (for _array_element_2 (`/Game/Core/Field/BP_MainField.SpawnedShips` (`/Game/Core/BP_GameState.BP_MainField` (`/Game/Core/BP_FunctionLibrary.Get Game State`)))
              (bind (_shipdata_shiptype _shipdata_coordinates) (break `/Game/Core/Ships/F_ShipData` (`/Game/Core/Ships/Blueprints/BP_ParentShip.ShipData` _array_element_2)))
              (if (`KismetArrayLibrary.Array_Contains` _shipdata_coordinates (`self.HittedPos`))
                (set `self.HittedShip` _array_element_2)
                (break)))
            (bind _output_get (set `self.DirectionToFire` (`|MakeArray` "Left" "Right" "Up" "Down" :!type "ETouchSwipeDirection Enum")))
            (`KismetArrayLibrary.Array_Shuffle` _output_get)
            (set `self.TempPos` (`self.HittedPos`))))))))

(fn `AI_Fire`
  (bind _pos (`self.GetNextCellToFire`))
  (if (`/Game/Core/BP_FunctionLibrary.PosIsValid` _pos)
    (bind _issuccessful (`/Game/Core/Field/BP_ParentField.Shot` (`/Game/Core/BP_GameState.BP_MainField` (`/Game/Core/BP_FunctionLibrary.Get Game State`)) _pos true))
    (if (not _issuccessful)
      (`KismetArrayLibrary.Array_Remove` (`self.DirectionToFire`) :!label _label)
      (set `self.TempPos` (`self.HittedPos`))
      (`self.AI_Fire`))
    (else
      (goto _label))))

(fn `GetNextCellToFire`
  (returns (Pos :type "Vector2D Structure"))
  (bind _asbp_battle_game_mode (cast `/Game/Core/BP_BattleGameMode` (`GameplayStatics.GetGameMode`)))
  (switch `/Game/Core/Enums/E_Difficulty` (`/Game/Core/BP_BattleGameMode.GameDifficulty` _asbp_battle_game_mode)
    (:`NewEnumerator0`
      _)
    (:`NewEnumerator2`
      (`self.HittedShip`
        (:`then`
          (bind _output_get (set `self.TempPos` (+ (`self.TempPos`) (select `ETouchSwipeDirection` (`|GetArrayItem` (`self.DirectionToFire`)) :`Left` (-1.0 0.0) :`Right` (1.0 0.0) :`Up` (0.0 -1.0) :`Down` (0.0 1.0) :!type "Vector2D Structure"))))
          (return _output_get))
        (:`else`
          _))))
  (bind _output_get_2 (set `self.NextCellPos` (`KismetMathLibrary.MakeVector2D` (`KismetMathLibrary.Conv_IntToDouble` (`KismetMathLibrary.RandomIntegerInRange` 0 9)) (`KismetMathLibrary.Conv_IntToDouble` (`KismetMathLibrary.RandomIntegerInRange` 0 9)))))
  (return _output_get_2))