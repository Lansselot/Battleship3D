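; Component that handles Battleship-style ship placement on a 10x10 BP_Field, by mouse or at random.
; A data table fills the ship kit, which is popped one ship at a time as the current ship.
; Each tick, a cursor trace snaps to a grid cell and previews a ghost, which input rotates or commits after validity checks.
; Random generation retries random cells and directions until remaining ships fit; clearing destroys ships and reloads the kit.
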(event `InputAction|Rotate`
  (params (Key :type "Key Structure"))
  ;[1 1 1] Inputs
  (:`Pressed`
    (`self.Rotate`)))

(event `InputAction|PlaceShip`
  (params (Key :type "Key Structure"))
  ;[1 1 1] Inputs
  (:`Pressed`
    (`self.PlaceShip`)))

(event `InputAction|GenerateRandom`
  (params (Key :type "Key Structure"))
  ;[1 1 1] Inputs
  (:`Pressed`
    (`self.Generate Random Pressed`)))

(event `InputAction|ClearField`
  (params (Key :type "Key Structure"))
  ;[1 1 1] Inputs
  (:`Pressed`
    (`self.ResetAllField`)))

(event `self.ReceiveBeginPlay`
  (`|ExecutionSequence`
    (:`then_0`
      (bind _shipkit (`self.ImportShipKit`))
      (set `self.Ship Kit` _shipkit))
    (:`then_1`
      (bind _next_ship_ship_type (`self.Pop Next Ship To Add`))
      (set `self.CurrentShip` _next_ship_ship_type))))

(event `PlaceGhost`
  (bind _positions (`/Game/Core/BP_FunctionLibrary.GetAllCordinatesFromFirst` (`self.CurrentShip`) (`self.CurrentPos`) (`self.CurrentDirection`)))
  (bind _bp_field (`self.BP_Field`)
    (:`then`
      (`/Game/Core/Field/BP_Field.PlaceShip` _bp_field (make `/Game/Core/Ships/F_ShipData` (`self.CurrentShip`) _positions) true))
    (:`else`)))

(event `self.ReceiveTick`
  (params (DeltaSeconds :type "Float (single-precision)"))
  (if (and (`|EnumInequality` (`self.CurrentShip`) "NewEnumerator4") (`self.MouseSelectEnable`))
    (bind _returnvalue (`self.Update Mouse Position`))
    (set `self.CurrentPos` _returnvalue)
    (`self.PlaceGhost`)))

(fn `Generate Random Pressed`
  (locals (pos :type "Array of Vector2D Structure"))
  (bind _currentship (`self.CurrentShip`))
  (if (not (`KismetArrayLibrary.Array_IsNotEmpty` (`self.Ship Kit`)))
    (`self.ResetAllField`))
  (if (`|EnumInequality` (`self.CurrentShip`) "NewEnumerator4") :!label _label
    (set `self.CurrentDirection` (cast `ETouchSwipeDirection` (`KismetMathLibrary.Conv_IntToByte` (`KismetMathLibrary.RandomIntegerInRange` 1 4))) :!label _label_2)
    (bind _positions (`/Game/Core/BP_FunctionLibrary.GetAllCordinatesFromFirst` (`self.CurrentShip`) (`KismetMathLibrary.MakeVector2D` (`KismetMathLibrary.Conv_IntToDouble` (`KismetMathLibrary.RandomIntegerInRange` 0 9)) (`KismetMathLibrary.Conv_IntToDouble` (`KismetMathLibrary.RandomIntegerInRange` 0 9))) (`self.CurrentDirection`)))
    (bind _output_get (set `local.pos` _positions))
    (if (and (`/Game/Core/Field/BP_Field.Possible To Place On Field` (`self.BP_Field`) (make `/Game/Core/Ships/F_ShipData` _currentship _output_get)) (`/Game/Core/BP_FunctionLibrary.PossibleToPlace` (make `/Game/Core/Ships/F_ShipData` _currentship _output_get)))
      (`/Game/Core/Field/BP_Field.PlaceShip` (`self.BP_Field`) (make `/Game/Core/Ships/F_ShipData` (`self.CurrentShip`) _output_get) false)
      (bind _next_ship_ship_type (`self.Pop Next Ship To Add`))
      (set `self.CurrentShip` _next_ship_ship_type)
      (goto _label)
      (else
        (goto _label_2)))
    (else
      (return))))

(fn `ImportShipKit`
  (returns (ShipKit :type "Array of /Game/Core/Ships/F_ShipKit Structure"))
  (locals (temp :type "/Game/Core/Ships/F_ShipKit Structure") (_ShipKit :type "Array of /Game/Core/Ships/F_ShipKit Structure"))
  (bind _datashipkit (`self.DataShipKit`))
  (bind _outrownames (`DataTableFunctionLibrary.GetDataTableRowNames` _datashipkit))
  (for _array_element _outrownames
    (bind _returnvalue (`|GetDataTableRow` _datashipkit _array_element)
      (:`then`
        (bind _output_get (set `local.temp` _returnvalue))
        (`KismetArrayLibrary.Array_Add` (`local._ShipKit`) _output_get))))
  (return (`local._ShipKit`)))

(fn `PlaceShip`
  (bind _currentship (`self.CurrentShip`))
  (if (`|EnumInequality` (`self.CurrentShip`) "NewEnumerator4")
    (bind _positions (`/Game/Core/BP_FunctionLibrary.GetAllCordinatesFromFirst` (`self.CurrentShip`) (`self.CurrentPos`) (`self.CurrentDirection`)))
    (bind _bp_field (`self.BP_Field`)
      (:`then`
        (if (and (`/Game/Core/Field/BP_Field.Possible To Place On Field` _bp_field (make `/Game/Core/Ships/F_ShipData` _currentship _positions)) (`/Game/Core/BP_FunctionLibrary.PossibleToPlace` (make `/Game/Core/Ships/F_ShipData` _currentship _positions)))
          (`/Game/Core/Field/BP_Field.PlaceShip` _bp_field (make `/Game/Core/Ships/F_ShipData` (`self.CurrentShip`) _positions) false)
          (bind _next_ship_ship_type (`self.Pop Next Ship To Add`))
          (set `self.CurrentShip` _next_ship_ship_type)))
      (:`else`))))

(fn `Pop Next Ship To Add`
  (returns (`Next Ship Ship Type` :type "/Game/Core/Ships/E_ShipType Enum"))
  (locals (NextShip :type "/Game/Core/Ships/F_ShipKit Structure"))
  (bind _nextship_shiptype (break `/Game/Core/Ships/F_ShipKit` (`local.NextShip`)))
  (bind (_nextship_shiptype_2 _nextship_amount) (break `/Game/Core/Ships/F_ShipKit` (`local.NextShip`)))
  (bind _ship_kit (`self.Ship Kit`))
  (bind _output (`|GetArrayItem` _ship_kit))
  (if (`KismetArrayLibrary.Array_IsNotEmpty` (`self.Ship Kit`))
    (bind _output_get (set `local.NextShip` _output))
    (`KismetArrayLibrary.Array_RemoveItem` _ship_kit _output)
    (if (> (`.Amount_3_ACAE5CCA46288F477620BDBC1BAEED0F` (break `/Game/Core/Ships/F_ShipKit` _output_get)) 1)
      (`KismetArrayLibrary.Array_Insert` (`self.Ship Kit`) (make `/Game/Core/Ships/F_ShipKit` _nextship_shiptype_2 (- _nextship_amount 1))))
    (return _nextship_shiptype)
    (else
      (return "NewEnumerator4"))))

(fn `ResetAllField`
  (bind _bp_field (`self.BP_Field`)
    (:`then`
      (`/Game/Core/Field/BP_Field.DestroyAllShips` _bp_field)
      (bind _shipkit (`self.ImportShipKit`))
      (set `self.Ship Kit` _shipkit)
      (bind _next_ship_ship_type (`self.Pop Next Ship To Add`))
      (set `self.CurrentShip` _next_ship_ship_type))
    (:`else`)))

(fn `Rotate`
  (set `self.CurrentDirection` (select `ETouchSwipeDirection` (`self.CurrentDirection`) :`None` "Left" :`Left` "Up" :`Right` "Down" :`Up` "Right" :`Down` "Left" :!type "ETouchSwipeDirection Enum"))
  (`self.PlaceGhost`))

(fn `Update Mouse Position`
  (returns (ReturnValue :type "Vector2D Structure"))
  (bind _ratio (`/Game/Core/BP_FunctionLibrary.GetRatio`))
  (bind (_worldlocation _worlddirection) (`PlayerController.DeprojectMousePositionToWorld` (`/Game/Core/BP_FunctionLibrary.Get Main Player Controller`)))
  (bind _outhit (`KismetSystemLibrary.LineTraceSingle` _worldlocation (+ _worldlocation (* _worlddirection 1000000.0)) "TraceTypeQuery1"))
  (bind (_bblockinghit _binitialoverlap _time _distance _location _impactpoint _normal _impactnormal _physmat _hitactor) (`GameplayStatics.BreakHitResult` _outhit))
  (bind _asbp_field (cast `/Game/Core/Field/BP_Field` _hitactor))
  (bind (_returnvalue_x _returnvalue_y) (`KismetMathLibrary.BreakVector` (- _location (`Actor.K2_GetActorLocation` _asbp_field))))
  (return (`KismetMathLibrary.MakeVector2D` (`KismetMathLibrary.Conv_IntToDouble` (`KismetMathLibrary.Clamp` (`KismetMathLibrary.Round` (/ _returnvalue_x _ratio)) 0 9)) (`KismetMathLibrary.Conv_IntToDouble` (`KismetMathLibrary.Clamp` (`KismetMathLibrary.Round` (/ _returnvalue_y _ratio)) 0 9)))))