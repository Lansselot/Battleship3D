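; BP_Field is the board for a battleship-style ship placement game, drawing a 10x10 grid and showing a ghost preview ship.
; The construction script builds the grid from scaled static mesh lines spaced by GetRatio.
; SetGhostShip replaces the current ghost, spawning the ship class for the given deck count at a location derived from its ship data.
; BeginPlay spawns a hardcoded two-deck ghost.
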(event `self.ReceiveBeginPlay`
  (`self.SetGhostShip` (make `/Game/Core/Ships/F_ShipData` "NewEnumerator1" (`|MakeArray` (2.0 2.0) (3.0 2.0) :!type "Vector2D Structure"))))

(event `SetGhostShip`
  (params (ShipData :type "/Game/Core/Ships/F_ShipData Structure"))
  (bind _ghostship (`self.GhostShip`)
    (:`then`
      (`self.K2_DestroyActor` _ghostship))
    (:`else`
      _))
  (bind _asbp_parent_ship (castclass `/Game/Core/Ships/Blueprints/BP_ParentShip` (select `/Game/Core/Ships/E_ShipType` (`.ShipType_2_10E763544A75E26FD0EEDA85F35DFDB0` (break `/Game/Core/Ships/F_ShipData` ShipData)) :`NewEnumerator0` "/Game/Core/Ships/Blueprints/BP_1DeckShip.BP_1DeckShip_C" :`NewEnumerator1` "/Game/Core/Ships/Blueprints/BP_2DeckShip.BP_2DeckShip_C" :`NewEnumerator2` "/Game/Core/Ships/Blueprints/BP_3DeckShip.BP_3DeckShip_C" :`NewEnumerator3` "/Game/Core/Ships/Blueprints/BP_4DeckShip.BP_4DeckShip_C" :!type "Actor Class Reference")))
  (bind _vector (`/Game/Core/BP_FunctionLibrary.GetLocationFromField` ShipData))
  (bind _returnvalue (`|SpawnActorFromClass` _asbp_parent_ship _vector "Undefined" "OverrideRootScale" null ShipData true null))
  (set `self.GhostShip` _returnvalue))

(fn `UserConstructionScript`
  (bind _returnvalue (* (`/Game/Core/BP_FunctionLibrary.GetRatio`) 5.0))
  (for _index (range 11)
    (`AddComponent|NODE_AddStaticMeshComponent-0` :`RelativeTransform` (`KismetMathLibrary.MakeTransform` (`KismetMathLibrary.MakeVector` (* _index (`/Game/Core/BP_FunctionLibrary.GetRatio`)) _returnvalue) (`KismetMathLibrary.MakeRotator` 0.0) (10.0 1000.0 10.0))))
  (for _index_2 (range 11)
    (`AddComponent|NODE_AddStaticMeshComponent-1` :`RelativeTransform` (`KismetMathLibrary.MakeTransform` (`KismetMathLibrary.MakeVector` _returnvalue (* _index_2 (`/Game/Core/BP_FunctionLibrary.GetRatio`))) (`KismetMathLibrary.MakeRotator` 0.0) (1000.0 10.0 10.0)))))