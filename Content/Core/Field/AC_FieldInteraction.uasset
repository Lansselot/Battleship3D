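; Actor component that handles player mouse and key interaction with the 10x10 game fields.
; Each tick, when mouse input is enabled, it traces from the cursor, converts the hit on a BP_ParentField into a clamped grid cell, and passes cell and direction to that field.
; Input actions rotate the placement direction, trigger the field action, and randomize or clear the main field during the Arranges game state.
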(event `InputAction|Rotate`
  (params (Key :type "Key Structure"))
  ;[1 1 1] Inputs
  (:`Pressed`
    (`self.Rotate`)))

(event `InputAction|Action`
  (params (Key :type "Key Structure"))
  ;[1 1 1] Inputs
  (:`Pressed`
    (bind _currentfield (`self.CurrentField`)
      (:`then`
        (`/Game/Core/Field/BP_ParentField.FieldAction` _currentfield (`self.CurrentPos`) (`self.CurrentDirection`)))
      (:`else`))))

(event `InputAction|GenerateRandom`
  (params (Key :type "Key Structure"))
  ;[1 1 1] Inputs
  (:`Pressed`
    (switch `/Game/Core/Enums/E_GameState` (`/Game/Core/BP_GameState.gameState` (`/Game/Core/BP_FunctionLibrary.Get Game State`))
      (:`NewEnumerator0`
        (bind _bp_mainfield (`/Game/Core/BP_GameState.BP_MainField` (`/Game/Core/BP_FunctionLibrary.Get Game State`))
          (:`then`
            (`/Game/Core/Field/BP_MainField.Generate Random` _bp_mainfield))
          (:`else`))))))

(event `InputAction|ClearField`
  (params (Key :type "Key Structure"))
  ;[1 1 1] Inputs
  (:`Pressed`
    (switch `/Game/Core/Enums/E_GameState` (`/Game/Core/BP_GameState.gameState` (`/Game/Core/BP_FunctionLibrary.Get Game State`))
      (:`NewEnumerator0`
        (bind _bp_mainfield (`/Game/Core/BP_GameState.BP_MainField` (`/Game/Core/BP_FunctionLibrary.Get Game State`))
          (:`then`
            (`/Game/Core/Field/BP_ParentField.ClearField` _bp_mainfield))
          (:`else`))))))

(event `self.ReceiveTick`
  (params (DeltaSeconds :type "Float (single-precision)"))
  (if (`self.MouseInputEnabled`)
    (bind (_field _vector2d) (`self.Update Mouse Position`))
    (bind _output_get (set `self.CurrentField` _field))
    (bind _output_get_2 (set `self.CurrentPos` _vector2d))
    (`/Engine/EditorBlueprintResources/StandardMacros.IsValid` _output_get
      (:`Is Valid`
        (`/Game/Core/Field/BP_ParentField.FieldSetCurrentPos` _output_get _output_get_2 (`self.CurrentDirection`)))
      (:`Is Not Valid`
        (bind _outactors (`GameplayStatics.GetAllActorsOfClass` "/Game/Core/Field/BP_ParentField.BP_ParentField_C"))
        (for _ _outactors
          _)))))

(fn `Rotate`
  (set `self.CurrentDirection` (select `ETouchSwipeDirection` (`self.CurrentDirection`) :`None` "Left" :`Left` "Up" :`Right` "Down" :`Up` "Right" :`Down` "Left" :!type "ETouchSwipeDirection Enum"))
  (bind _currentfield (`self.CurrentField`)
    (:`then`
      (`/Game/Core/Field/BP_ParentField.FieldSetCurrentPos` _currentfield (`self.CurrentPos`) (`self.CurrentDirection`)))
    (:`else`)))

(fn `Update Mouse Position`
  (returns (Field :type "/Game/Core/Field/BP_ParentField Object Reference") (Vector2D :type "Vector2D Structure"))
  (bind _ratio (`/Game/Core/BP_FunctionLibrary.GetRatio`))
  (bind (_worldlocation _worlddirection) (`PlayerController.DeprojectMousePositionToWorld` (`/Game/Core/BP_FunctionLibrary.Get Main Player Controller`)))
  (bind _outhit (`KismetSystemLibrary.LineTraceSingle` :`Start` _worldlocation :`End` (+ _worldlocation (* _worlddirection 1000000.0)) :`TraceChannel` "TraceTypeQuery3" :`DrawDebugType` "ForOneFrame"))
  (bind (_bblockinghit _binitialoverlap _time _distance _location _impactpoint _normal _impactnormal _physmat _hitactor) (`GameplayStatics.BreakHitResult` _outhit))
  (bind _asbp_parent_field (cast `/Game/Core/Field/BP_ParentField` _hitactor)
    (:`then`
      (bind (_x _y) (`KismetMathLibrary.BreakVector3f` (`KismetMathLibrary.InverseTransformLocation` (`Actor.GetTransform` _hitactor) _location)))
      (return _asbp_parent_field (`KismetMathLibrary.MakeVector2D` (`KismetMathLibrary.Conv_IntToDouble` (`KismetMathLibrary.Clamp` (`KismetMathLibrary.FFloor` (/ _x _ratio)) 0 9)) (`KismetMathLibrary.Conv_IntToDouble` (`KismetMathLibrary.Clamp` (`KismetMathLibrary.FFloor` (/ _y _ratio)) 0 9)))))
    (:`CastFailed`
      (return null (0.0 0.0)))))