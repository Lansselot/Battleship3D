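; Base Battleship field that builds a grid from static meshes and tracks ships, filled cells and shot cells, leaving field input actions to children.
; A data-table ship kit feeds the current ship, which random generation places by retrying until it fits without touching others.
; Shots remove filled cells and report hits.
; UpdateShips detects sunk ships, auto-shoots their neighbours, spawns attached ship actors and signals when all are destroyed.
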(event `self.ReceiveBeginPlay`
  (`|ExecutionSequence`
    (:`then_0`
      (bind _shipkit (`self.ImportShipKit`))
      (set `self.Ship Kit` _shipkit))
    (:`then_1`
      (bind _next_ship_ship_type (`self.Pop Next Ship To Add`))
      (`self.SetCurrentShip` _next_ship_ship_type))))

(fn `ClearField`
  (`KismetArrayLibrary.Array_Clear` (`self.FilledCells`))
  (bind _shipkit (`self.ImportShipKit`))
  (set `self.Ship Kit` _shipkit)
  (bind _next_ship_ship_type (`self.Pop Next Ship To Add`))
  (`self.SetCurrentShip` _next_ship_ship_type))

(fn `FieldAction`
  (params (Position :type "Vector2D Structure") (Direction :type "ETouchSwipeDirection Enum" :default "None"))
  (`KismetSystemLibrary.PrintString` "Error: Function not implemented" true true (struct :`R` 1.0 :`A` 1.0) 10.0))

(fn `FieldSetCurrentPos`
  (params (Position :type "Vector2D Structure") (Direction :type "ETouchSwipeDirection Enum" :default "None"))
  (`KismetSystemLibrary.PrintString` "Error: Function not implemented" true true (struct :`R` 1.0 :`A` 1.0) 10.0))

(fn `Generate Random`
  (locals (pos :type "Array of Vector2D Structure") (CurrentDirection :type "ETouchSwipeDirection Enum") (Ships_ :type "Array of /Game/Core/Ships/F_ShipData Structure"))
  (bind _currentship (`self.CurrentShip`))
  (if (not (`KismetArrayLibrary.Array_IsNotEmpty` (`self.Ship Kit`)))
    (`self.ClearField`))
  (if (`|EnumInequality` (`self.CurrentShip`) "NewEnumerator4") :!label _label
    (set `local.CurrentDirection` (cast `ETouchSwipeDirection` (`KismetMathLibrary.Conv_IntToByte` (`KismetMathLibrary.RandomIntegerInRange` 1 4))) :!label _label_2)
    (bind _positions (`/Game/Core/BP_FunctionLibrary.GetAllCordinatesFromFirst` (`self.CurrentShip`) (`KismetMathLibrary.MakeVector2D` (`KismetMathLibrary.Conv_IntToDouble` (`KismetMathLibrary.RandomIntegerInRange` 0 9)) (`KismetMathLibrary.Conv_IntToDouble` (`KismetMathLibrary.RandomIntegerInRange` 0 9))) (`local.CurrentDirection`)))
    (bind _output_get (set `local.pos` _positions))
    (if (and (`self.Possible To Place On Field` (make `/Game/Core/Ships/F_ShipData` _currentship _output_get)) (`/Game/Core/BP_FunctionLibrary.PossibleToPlace` (make `/Game/Core/Ships/F_ShipData` _currentship _output_get)))
      (`self.PlaceShip` (make `/Game/Core/Ships/F_ShipData` (`self.CurrentShip`) _output_get))
      (bind _next_ship_ship_type (`self.Pop Next Ship To Add`))
      (`self.SetCurrentShip` _next_ship_ship_type)
      (goto _label)
      (else
        (goto _label_2)))
    (else
      (return))))

(fn `Get Location from Field`
  (params (Vector2D :type "Vector2D Structure"))
  (returns (Transform :type "Transform Structure"))
  (bind (_returnvalue_location _returnvalue_rotation _returnvalue_scale) (`KismetMathLibrary.BreakTransform` (`self.GetTransform`)))
  (return (`KismetMathLibrary.MakeTransform` (`KismetMathLibrary.MakeVector` (* (+ Vector2D_X 0.5) 1.0 10000.0) (* (+ Vector2D_Y 0.5) 10000.0 1.0)) (struct) _returnvalue_scale)))

(fn `Get Ship Location from Field`
  (params (ShipData :type "/Game/Core/Ships/F_ShipData Structure"))
  (returns (Transform :type "Transform Structure"))
  (locals (Mean_X :type "Float (double-precision)") (Mean_Y :type "Float (double-precision)"))
  (bind _returnvalue (`KismetArrayLibrary.Array_Length` ShipData_Coordinates_8_A8CB159A4E88E5750AA655A5CC42942B))
  (bind _output_x (`KismetMathLibrary.BreakVector2D` (`|GetArrayItem` ShipData_Coordinates_8_A8CB159A4E88E5750AA655A5CC42942B)))
  (for _array_element ShipData_Coordinates_8_A8CB159A4E88E5750AA655A5CC42942B
    (bind (_x _y) (`KismetMathLibrary.BreakVector2D` _array_element))
    (set `local.Mean_X` (+ (`local.Mean_X`) _x))
    (set `local.Mean_Y` (+ (`local.Mean_Y`) _y)))
  (bind _output_get (set `local.Mean_X` (/ (`local.Mean_X`) _returnvalue)))
  (bind _output_get_2 (set `local.Mean_Y` (/ (`local.Mean_Y`) _returnvalue)))
  (bind (_transform_location _transform_rotation _transform_scale) (`KismetMathLibrary.BreakTransform` (`self.Get Location from Field` (`KismetMathLibrary.MakeVector2D` _output_get _output_get_2))))
  (return (`KismetMathLibrary.MakeTransform` _transform_location (`KismetMathLibrary.MakeRotator` 0.0 0.0 (`KismetMathLibrary.SelectFloat` 90.0 0.0 (== (`local.Mean_X`) _output_x))) _transform_scale)))

(fn `GetNeighbours`
  (params (F_ShipData :type "/Game/Core/Ships/F_ShipData Structure (by ref)"))
  (returns (Neighbours :type "Array of Vector2D Structure"))
  (locals (DeltaNeighbours :type "Array of Vector2D Structure") (Neighbours_ :type "Array of Vector2D Structure"))
  (bind (_shiptype _coordinates) (break `/Game/Core/Ships/F_ShipData` F_ShipData))
  (for _array_element _coordinates
    (for _array_element_2 (`local.DeltaNeighbours`)
      (`KismetArrayLibrary.Array_Add` (`local.Neighbours_`) (+ _array_element_2 _array_element))))
  (for _array_element_3 _coordinates
    (`KismetArrayLibrary.Array_AddUnique` (`local.Neighbours_`) _array_element_3))
  (return (`local.Neighbours_`)))

(fn `ImportShipKit`
  (returns (ShipKit :type "Array of /Game/Core/Ships/F_ShipKit Structure"))
  (locals (temp :type "/Game/Core/Ships/F_ShipKit Structure") (_ShipKit :type "Array of /Game/Core/Ships/F_ShipKit Structure"))
  (bind _datashipkit (`self.DataShipKit`))
  (bind _outrownames (`DataTableFunctionLibrary.GetDataTableRowNames` _datashipkit))
  (for _array_element _outrownames
    (bind _returnvalue (`|GetDataTableRow` _datashipkit _array_element)
      (:`then`
        (bind _output_get (set `local.temp` _returnvalue))
        (`KismetArrayLibrary.Array_Add` (`local._ShipKit`) _output_get))))
  (return (`local._ShipKit`)))

(fn `PlaceShip`
  (params (ShipData :type "/Game/Core/Ships/F_ShipData Structure") (`Ghost?` :type Boolean))
  (if (not `Ghost?`)
    (`KismetArrayLibrary.Array_Append` (`self.FilledCells`) (`.Coordinates_8_A8CB159A4E88E5750AA655A5CC42942B` (break `/Game/Core/Ships/F_ShipData` ShipData)))
    (`KismetArrayLibrary.Array_Add` (`self.Ships`) ShipData)))

(fn `Pop Next Ship To Add`
  (returns (`Next Ship Ship Type` :type "/Game/Core/Enums/E_ShipType Enum"))
  (locals (NextShip :type "/Game/Core/Ships/F_ShipKit Structure"))
  (bind _ship_kit (`self.Ship Kit`))
  (bind _nextship_shiptype (break `/Game/Core/Ships/F_ShipKit` (`local.NextShip`)))
  (bind (_nextship_shiptype_2 _nextship_amount) (break `/Game/Core/Ships/F_ShipKit` (`local.NextShip`)))
  (bind _output (`|GetArrayItem` _ship_kit))
  (if (`KismetArrayLibrary.Array_IsNotEmpty` (`self.Ship Kit`))
    (bind _output_get (set `local.NextShip` _output))
    (`KismetArrayLibrary.Array_RemoveItem` _ship_kit _output)
    (if (> (`.Amount_3_ACAE5CCA46288F477620BDBC1BAEED0F` (break `/Game/Core/Ships/F_ShipKit` _output_get)) 1)
      (`KismetArrayLibrary.Array_Insert` (`self.Ship Kit`) (make `/Game/Core/Ships/F_ShipKit` _nextship_shiptype_2 (- _nextship_amount 1))))
    (return _nextship_shiptype)
    (else
      (return "NewEnumerator4"))))

(fn `Possible To Place On Field`
  (params (F_ShipData :type "/Game/Core/Ships/F_ShipData Structure (by ref)"))
  (returns (ReturnValue :type Boolean))
  (locals (DeltaNeighbours :type "Array of Vector2D Structure"))
  (bind _neighbours (`self.GetNeighbours` F_ShipData))
  (for _array_element _neighbours
    (if (`KismetArrayLibrary.Array_Contains` (`self.FilledCells`) _array_element)
      (return false)))
  (return true))

(fn `SetCurrentShip`
  (params (CurrentShip :type "/Game/Core/Enums/E_ShipType Enum" :default "NewEnumerator4"))
  (returns (Output_Get :type "/Game/Core/Enums/E_ShipType Enum"))
  (bind _output_get (set `self.CurrentShip` CurrentShip))
  (if (`|EnumInequality` _output_get "NewEnumerator4")
    (return _output_get)
    (else
      (`self.OnAllShipsPlaced`)
      (return "NewEnumerator4"))))

(fn `Shot`
  (params (Pos :type "Vector2D Structure") (byPlayer :type Boolean))
  (returns (IsSuccessful :type Boolean) (`Hit?` :type Boolean))
  (if (`/Game/Core/BP_FunctionLibrary.PosIsValid` Pos)
    (if (`KismetArrayLibrary.Array_Contains` (`self.CheckedCells`) Pos)
      _
      (else
        (`KismetArrayLibrary.Array_Add` (`self.CheckedCells`) Pos)
        (bind _returnvalue (`KismetArrayLibrary.Array_RemoveItem` (`self.FilledCells`) Pos))
        (if byPlayer
          (`self.OnShot` self _returnvalue))
        (return true _returnvalue))))
  (return false false))

(fn `Update Ships`
  (returns (ShipDestroyed :type Boolean) (F_ShipData :type "/Game/Core/Ships/F_ShipData Structure"))
  (locals (_ShipDestroyed :type Boolean) (Ship :type "/Game/Core/Ships/F_ShipData Structure"))
  (bind _ship (`local.Ship`))
  (for _array_element (`self.Ships`)
    (set `local.Ship` _array_element)
    (set `local._ShipDestroyed` true)
    (for _array_element_2 (`.Coordinates_8_A8CB159A4E88E5750AA655A5CC42942B` (break `/Game/Core/Ships/F_ShipData` (`local.Ship`)))
      (if (not (`KismetArrayLibrary.Array_Contains` (`self.CheckedCells`) _array_element_2))
        (set `local._ShipDestroyed` false)))
    (if (`local._ShipDestroyed`)
      (bind _neighbours (`self.GetNeighbours` _ship))
      (for _array_element_3 _neighbours
        (`self.Shot` _array_element_3))
      (bind _asbp_parent_ship (castclass `/Game/Core/Ships/Blueprints/BP_ParentShip` (select `/Game/Core/Enums/E_ShipType` (`.ShipType_2_10E763544A75E26FD0EEDA85F35DFDB0` (break `/Game/Core/Ships/F_ShipData` _ship)) :`NewEnumerator0` "/Game/Core/Ships/Blueprints/BP_1DeckShip.BP_1DeckShip_C" :`NewEnumerator1` "/Game/Core/Ships/Blueprints/BP_2DeckShip.BP_2DeckShip_C" :`NewEnumerator2` "/Game/Core/Ships/Blueprints/BP_3DeckShip.BP_3DeckShip_C" :`NewEnumerator3` "/Game/Core/Ships/Blueprints/BP_4DeckShip.BP_4DeckShip_C" :!type "Actor Class Reference")))
      (bind _returnvalue (`|SpawnActorFromClass` _asbp_parent_ship (`self.Get Ship Location from Field` _ship) "Undefined" "OverrideRootScale" null _ship "NewEnumerator3" null))
      (`self.K2_AttachToActor` _returnvalue self "None" "KeepRelative" "KeepRelative" "KeepWorld" true)
      (`KismetArrayLibrary.Array_RemoveItem` (`self.Ships`) _ship)
      (if (`KismetArrayLibrary.Array_IsEmpty` (`self.Ships`))
        (`self.OnAllShipsDestroyed`))
      (return true _ship)))
  (return false))

(fn `UserConstructionScript`
  (bind _returnvalue (* (`/Game/Core/BP_FunctionLibrary.GetRatio`) 5.0))
  (bind _returnvalue_2 (* (`/Game/Core/BP_FunctionLibrary.GetRatio`) 5.0))
  (for _index (range 11)
    (`AddComponent|NODE_AddStaticMeshComponent-3` :`RelativeTransform` (`KismetMathLibrary.MakeTransform` (`KismetMathLibrary.MakeVector` (* _index (`/Game/Core/BP_FunctionLibrary.GetRatio`)) _returnvalue) (`KismetMathLibrary.MakeRotator` 0.0) (10.0 1000.0 10.0))))
  (for _index_2 (range 11)
    (`AddComponent|NODE_AddStaticMeshComponent-4` :`RelativeTransform` (`KismetMathLibrary.MakeTransform` (`KismetMathLibrary.MakeVector` _returnvalue (* _index_2 (`/Game/Core/BP_FunctionLibrary.GetRatio`))) (`KismetMathLibrary.MakeRotator` 0.0) (1000.0 10.0 10.0))))
  (`AddComponent|NODE_AddStaticMeshComponent-5` :`RelativeTransform` (`KismetMathLibrary.MakeTransform` (`KismetMathLibrary.MakeVector` _returnvalue_2 _returnvalue_2) (`KismetMathLibrary.MakeRotator` 0.0) (1400.0 1400.0 0.0))))