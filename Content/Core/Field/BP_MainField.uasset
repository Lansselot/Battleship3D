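; Battleship field Blueprint that handles ship placement during the Arranges game state and shows shot results, extending a parent field class.
; Position and direction updates respawn a ghost ship whose state reflects placement validity.
; Field actions spawn and track valid ships, then advance to the next ship, while clearing destroys tracked ships.
; Successful shots reuse one-deck ship actors as markers, with state set by hit or miss.
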(event `self.ReceiveBeginPlay`
  (`parent.ReceiveBeginPlay`))

(fn `ClearField`
  (`parent.ClearField`)
  (for _array_element (`self.SpawnedShips`)
    (`self.K2_DestroyActor` _array_element))
  (`KismetArrayLibrary.Array_Clear` (`self.SpawnedShips`))
  (`KismetArrayLibrary.Array_Clear` (`self.FilledCells`)))

(fn `FieldAction`
  (params (Position :type "Vector2D Structure") (Direction :type "ETouchSwipeDirection Enum" :default "None"))
  (bind _currentship (`self.CurrentShip`))
  (bind _positions (`/Game/Core/BP_FunctionLibrary.GetAllCordinatesFromFirst` (`self.CurrentShip`) Position Direction))
  (if (and (`self.Possible To Place On Field` (make `/Game/Core/Ships/F_ShipData` _currentship _positions)) (`/Game/Core/BP_FunctionLibrary.PossibleToPlace` (make `/Game/Core/Ships/F_ShipData` _currentship _positions)))
    (`self.PlaceShip` (make `/Game/Core/Ships/F_ShipData` (`self.CurrentShip`) _positions))
    (bind _next_ship_ship_type (`self.Pop Next Ship To Add`))
    (`self.SetCurrentShip` _next_ship_ship_type)))

(fn `FieldSetCurrentPos`
  (params (Position :type "Vector2D Structure") (Direction :type "ETouchSwipeDirection Enum" :default "None"))
  (if (or (!= Position (`self.GhostPos`)) (`|EnumInequality` Direction (`self.GhostRotate`)))
    (bind _output_get (set `self.GhostRotate` Direction))
    (bind _output_get_2 (set `self.GhostPos` Position))
    (bind _positions (`/Game/Core/BP_FunctionLibrary.GetAllCordinatesFromFirst` (`self.CurrentShip`) _output_get_2 _output_get))
    (`self.PlaceShip` (make `/Game/Core/Ships/F_ShipData` (`self.CurrentShip`) _positions) true)))

(fn `PlaceShip`
  (params (ShipData :type "/Game/Core/Ships/F_ShipData Structure") (`Ghost?` :type Boolean))
  (bind (_transform_location _transform_rotation _transform_scale) (`KismetMathLibrary.BreakTransform` (`self.Get Ship Location from Field` ShipData)))
  (`parent.PlaceShip` ShipData `Ghost?`)
  (switch `/Game/Core/Enums/E_GameState` (`/Game/Core/BP_GameState.gameState` (`/Game/Core/BP_FunctionLibrary.Get Game State`))
    (:`NewEnumerator0`
      (bind _ghostship (`self.GhostShip`)
        (:`then`
          (`self.K2_DestroyActor` _ghostship))
        (:`else`
          _))
      (bind _asbp_parent_ship (castclass `/Game/Core/Ships/Blueprints/BP_ParentShip` (select `/Game/Core/Enums/E_ShipType` (`.ShipType_2_10E763544A75E26FD0EEDA85F35DFDB0` (break `/Game/Core/Ships/F_ShipData` ShipData)) :`NewEnumerator0` "/Game/Core/Ships/Blueprints/BP_1DeckShip.BP_1DeckShip_C" :`NewEnumerator1` "/Game/Core/Ships/Blueprints/BP_2DeckShip.BP_2DeckShip_C" :`NewEnumerator2` "/Game/Core/Ships/Blueprints/BP_3DeckShip.BP_3DeckShip_C" :`NewEnumerator3` "/Game/Core/Ships/Blueprints/BP_4DeckShip.BP_4DeckShip_C" :!type "Actor Class Reference")))
      (bind _returnvalue (`|SpawnActorFromClass` _asbp_parent_ship (`KismetMathLibrary.MakeTransform` _transform_location _transform_rotation _transform_scale) "Undefined" "OverrideRootScale" null ShipData (select `bool` `Ghost?` :`false` "NewEnumerator0" :`true` (select `bool` (and (`/Game/Core/BP_FunctionLibrary.PossibleToPlace` ShipData) (`self.Possible To Place On Field` ShipData)) :`false` "NewEnumerator2" :`true` "NewEnumerator1" :!type "/Game/Core/Enums/E_ShipState Enum")) null))
      (if `Ghost?`
        (set `self.GhostShip` _returnvalue)
        (else
          (`KismetArrayLibrary.Array_Add` (`self.SpawnedShips`) _returnvalue))))))

(fn `SetCurrentShip`
  (params (CurrentShip :type "/Game/Core/Enums/E_ShipType Enum" :default "NewEnumerator4"))
  (returns (Output_Get :type "/Game/Core/Enums/E_ShipType Enum"))
  (bind _output_get (`parent.SetCurrentShip` CurrentShip))
  (bind _output_get_2 (set `self.CurrentShip` CurrentShip))
  (if (`|EnumInequality` _output_get_2 "NewEnumerator4")
    (`self.FieldSetCurrentPos` (`self.GhostPos`) (`self.GhostRotate`))
    (bind _positions (`/Game/Core/BP_FunctionLibrary.GetAllCordinatesFromFirst` (`self.CurrentShip`) (`self.GhostPos`) (`self.GhostRotate`)))
    (`self.PlaceShip` (make `/Game/Core/Ships/F_ShipData` (`self.CurrentShip`) _positions) true)
    (return _output_get)))

(fn `Shot`
  (params (Pos :type "Vector2D Structure") (byPlayer :type Boolean))
  (returns (IsSuccessful :type Boolean) (`Hit?` :type Boolean))
  (bind _f_shipdata (make `/Game/Core/Ships/F_ShipData` "NewEnumerator0" (`|MakeArray` Pos)))
  (bind (_issuccessful _hit_) (`parent.Shot` Pos byPlayer))
  (if _issuccessful
    (`|SpawnActorFromClass` "/Game/Core/Ships/Blueprints/BP_1DeckShip.BP_1DeckShip_C" (`self.Get Ship Location from Field` _f_shipdata) "Undefined" "OverrideRootScale" null _f_shipdata (select `bool` _hit_ :`false` "NewEnumerator2" :`true` "NewEnumerator1" :!type "/Game/Core/Enums/E_ShipState Enum") null))
  (return _issuccessful _hit_))

(fn `UserConstructionScript`
  (`parent.UserConstructionScript`))