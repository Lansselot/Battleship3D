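; BP_EnemyField is the enemy's field, a child Blueprint that adds targeting and shooting to inherited field logic.
; BeginPlay calls GenerateRandomPressed and iterates the result with an empty loop body, leaving a debug print disconnected.
; FieldSetCurrentPos replaces the BP_Target marker whenever the selected position changes, placing it via GetLocationFromField.
; FieldAction fires Shot at the given position; both functions ignore Direction.
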(event `self.ReceiveBeginPlay`
  (`parent.ReceiveBeginPlay`)
  (bind _filledcells (`self.Generate Random Pressed`))
  (for _array_element _filledcells
    _))

(fn `FieldAction`
  (params (Position :type "Vector2D Structure") (Direction :type "ETouchSwipeDirection Enum" :default "None"))
  (`self.Shot` Position))

(fn `FieldSetCurrentPos`
  (params (Position :type "Vector2D Structure") (Direction :type "ETouchSwipeDirection Enum" :default "None"))
  (bind (_transform_location _transform_rotation _transform_scale) (`KismetMathLibrary.BreakTransform` (`self.Get Location from Field` Position)))
  (if (!= Position (`self.TargetPos`))
    (bind _bp_target (`self.BP_Target`)
      (:`then`
        (`self.K2_DestroyActor` _bp_target))
      (:`else`
        _))
    (bind _returnvalue (`|SpawnActorFromClass` "/Game/Core/Target/BP_Target.BP_Target_C" (`KismetMathLibrary.MakeTransform` _transform_location _transform_rotation _transform_scale) "Undefined" "OverrideRootScale" null null))
    (set `self.BP_Target` _returnvalue)
    (set `self.TargetPos` Position)))

(fn `UserConstructionScript`
  (`parent.UserConstructionScript`))