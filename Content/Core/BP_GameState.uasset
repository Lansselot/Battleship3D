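; BP_GameState sets up the boards for a ship placement game, judging by its field and event names.
; On BeginPlay it spawns BP_MainField, offset along X by GetRatio, hands it to the player controller's AC_FieldInteraction and binds to its AllShipsPlaced event.
; ShipsPlaced spawns BP_EnemyField on the opposite side and passes it to the same component.
; Init_HUD is empty, and the WBP_HUD creation code is disconnected.
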(event `self.ReceiveBeginPlay`
  (`self.InitField`))

(event `Init_HUD`)

(event `InitField`
  (bind _returnvalue (`self.GetComponentByClass` (`/Game/Core/BP_FunctionLibrary.Get Main Player Controller`) "/Game/Core/Field/AC_FieldInteraction.AC_FieldInteraction_C"))
  (bind _returnvalue_2 (`|SpawnActorFromClass` "/Game/Core/Field/BP_MainField.BP_MainField_C" (`KismetMathLibrary.MakeTransform` (`KismetMathLibrary.MakeVector` (* (`/Game/Core/BP_FunctionLibrary.GetRatio`) -12.5))) "Undefined" "OverrideRootScale" null null))
  (`/Engine/EditorBlueprintResources/StandardMacros.IsValid` _returnvalue
    (:`Is Valid`
      (bind _output_get (set `/Game/Core/Field/AC_FieldInteraction.BP_MainField` _returnvalue_2 _returnvalue))
      (add `/Game/Core/Field/BP_MainField.AllShipsPlaced` _output_get (`|CreateDelegate` :!event `ShipsPlaced`)))))

(event `ShipsPlaced`
  (bind _returnvalue (`self.GetComponentByClass` (`/Game/Core/BP_FunctionLibrary.Get Main Player Controller`) "/Game/Core/Field/AC_FieldInteraction.AC_FieldInteraction_C"))
  (bind _returnvalue_2 (`|SpawnActorFromClass` "/Game/Core/Field/BP_EnemyField.BP_EnemyField_C" (`KismetMathLibrary.MakeTransform` (`KismetMathLibrary.MakeVector` (* (`/Game/Core/BP_FunctionLibrary.GetRatio`) 12.5))) "Undefined" "OverrideRootScale" null null))
  (`/Engine/EditorBlueprintResources/StandardMacros.IsValid` _returnvalue
    (:`Is Valid`
      (set `/Game/Core/Field/AC_FieldInteraction.BP_EnemyField` _returnvalue_2 _returnvalue))))

(fn `UserConstructionScript`)