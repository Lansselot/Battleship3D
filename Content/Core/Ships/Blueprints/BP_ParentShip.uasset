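; BP_ParentShip is a parent ship Blueprint that shows whether the ship can be placed through a colored ghost material.
; On BeginPlay it switches on ShipState and applies M_GhostMaterial to the Ship0 component.
; A dynamic material instance then sets the Color parameter to green for possible placement or red for impossible placement.
; The state is read only at BeginPlay, with no updates afterward in this graph.
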(event `self.ReceiveBeginPlay`
  (bind _ship_0 (`self.Ship_0`))
  (bind _ship_0_2 (`self.Ship_0`))
  (bind _returnvalue (`PrimitiveComponent.GetMaterial` _ship_0 0))
  (switch `/Game/Core/Enums/E_ShipState` (`self.ShipState`)
    (:`NewEnumerator1`
      (`PrimitiveComponent.SetMaterial` _ship_0 0 "/Game/Assets/Materials/M_GhostMaterial.M_GhostMaterial")
      (bind _returnvalue_2 (`PrimitiveComponent.CreateDynamicMaterialInstance` _ship_0_2 0 _returnvalue "None"))
      (`MaterialInstanceDynamic.SetVectorParameterValue` _returnvalue_2 "Color" (struct :`G` 1.0 :`A` 1.0)))
    (:`NewEnumerator2`
      (`PrimitiveComponent.SetMaterial` _ship_0 0 "/Game/Assets/Materials/M_GhostMaterial.M_GhostMaterial")
      (bind _returnvalue_3 (`PrimitiveComponent.CreateDynamicMaterialInstance` _ship_0_2 0 _returnvalue "None"))
      (`MaterialInstanceDynamic.SetVectorParameterValue` _returnvalue_3 "Color" (struct :`R` 1.0 :`A` 1.0)))))

(fn `UserConstructionScript`)