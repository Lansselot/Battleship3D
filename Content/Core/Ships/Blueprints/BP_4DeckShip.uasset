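; BP_4DeckShip is a four-deck ship Blueprint, a child class that supplies the meshes for this ship size.
; Its construction script runs the parent's, then sets the Ship mesh to the wrecked or intact model based on the ShipState enum.
; The event graph holds only disabled default events, so this Blueprint adds no runtime logic of its own.
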(fn `UserConstructionScript`
  (`parent.UserConstructionScript`)
  (`StaticMeshComponent.SetStaticMesh` (`self.Ship`) (select `bool` (`|EnumEquality` (`self.ShipState`) "NewEnumerator3") :`false` "/Game/Assets/Ships/4deck/4_Ship.4_Ship" :`true` "/Game/Assets/Ships/4deck/4_Ship_wrecked.4_Ship_wrecked" :!type "StaticMesh Object Reference")))